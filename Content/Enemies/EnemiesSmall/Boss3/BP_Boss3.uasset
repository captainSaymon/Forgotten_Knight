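; BP_Boss3 is the third boss enemy, a child Blueprint that adds its own on-screen health bar to inherited behavior.
; On BeginPlay it runs the parent logic, then creates and caches a WBP_HealthBarBoss3 widget from a class variable.
; The PrzelaczPasekBossa override calls the parent, then adds the bar to the viewport with a debug print, or removes it, based on the Pokazac flag.
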(event EventBeginPlay
  (|CallParentFunction)
  (bind _returnvalue (UserInterface|CreateWidget (Variables|Default|GetKlasaPaskaBossa3)))
  (bind _aswbp_health_bar_boss_3 (Utilities|Casting|CastToWBP_HealthBarBoss3 _returnvalue))
  (Variables|Default|SetPasekNaEkranieBossa3 _aswbp_health_bar_boss_3))

(event Collision|EventActorBeginOverlap
  (params (OtherActor :type Actor%20Object%20Reference))
  (|CallParentFunction OtherActor) ; Ten węzeł jest wyłączony i nie będzie wywoływany.\nPrzeciągnij gniazda, aby utworzyć funkcjonalność.
)

(event EventTick
  (params (DeltaSeconds :type Float%20%28single-precision%29))
  (|CallParentFunction DeltaSeconds) ; Ten węzeł jest wyłączony i nie będzie wywoływany.\nPrzeciągnij gniazda, aby utworzyć funkcjonalność.
)

(fn ConstructionScript
  (|CallParentFunction))

(fn PrzelaczPasekBossa
  (params (Pokazac :type Boolean))
  (bind _paseknaekraniebossa3 (Variables|Default|GetPasekNaEkranieBossa3))
  (|CallParentFunction Pokazac)
  (if Pokazac
    (UserInterface|Viewport|AddtoViewport _paseknaekraniebossa3 0)
    (Development|PrintString "FUNKCJA WYSWIETLANIA PASK")
    (else
      (Widget|RemovefromParent _paseknaekraniebossa3))))