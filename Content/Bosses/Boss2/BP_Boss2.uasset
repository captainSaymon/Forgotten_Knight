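; Boss 2 Blueprint that manages the on-screen health bar for the second boss.
; On BeginPlay it runs the parent logic, then creates a WBP_HealthBarBoss2 widget and caches it without displaying it.
; The PrzelaczPasekBossa (toggle boss bar) override calls the parent, then adds the widget to the viewport with a debug print or removes it, based on the Pokazac (show) flag.
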(event EventBeginPlay
  (|CallParentFunction)
  (bind _returnvalue (UserInterface|CreateWidget (Variables|Default|GetKlasaPaskaBossa2)))
  (bind _aswbp_health_bar_boss_2 (Utilities|Casting|CastToWBP_HealthBarBoss2 _returnvalue))
  (Variables|Default|SetPasekNaEkranieBossa2 _aswbp_health_bar_boss_2))

(event Collision|EventActorBeginOverlap
  (params (OtherActor :type Actor%20Object%20Reference))
  (|CallParentFunction OtherActor) ; Ten węzeł jest wyłączony i nie będzie wywoływany.\nPrzeciągnij gniazda, aby utworzyć funkcjonalność.
)

(fn ConstructionScript
  (|CallParentFunction))

(fn PrzelaczPasekBossa
  (params (Pokazac :type Boolean))
  (bind _paseknaekraniebossa2 (Variables|Default|GetPasekNaEkranieBossa2))
  (|CallParentFunction Pokazac)
  (if Pokazac
    (UserInterface|Viewport|AddtoViewport _paseknaekraniebossa2 0)
    (Development|PrintString "FUNKCJA WYSWIETLANIA PASKA")
    (else
      (Widget|RemovefromParent _paseknaekraniebossa2))))