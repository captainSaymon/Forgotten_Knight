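; BP_Boss1 is a boss enemy Blueprint that puts a boss bar widget on screen when play begins.
; BeginPlay runs the parent logic, creates a widget from KlasaPaskaBossa and adds it to the viewport.
; The PasekNaEkranieBossa variable is set to None rather than to the new widget, so no reference is stored there.
; Overlap and Tick are disabled stubs, and the construction script only calls the parent.
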(event EventBeginPlay
  (|CallParentFunction)
  (bind _returnvalue (UserInterface|CreateWidget (Variables|Default|GetKlasaPaskaBossa)))
  (Variables|Default|SetPasekNaEkranieBossa 0)
  (UserInterface|Viewport|AddtoViewport _returnvalue 0))

(event Collision|EventActorBeginOverlap
  (params (OtherActor :type Actor%20Object%20Reference))
  (|CallParentFunction OtherActor) ; Ten węzeł jest wyłączony i nie będzie wywoływany.\nPrzeciągnij gniazda, aby utworzyć funkcjonalność.
)

(event EventTick
  (params (DeltaSeconds :type Float%20%28single-precision%29))
  (|CallParentFunction DeltaSeconds) ; Ten węzeł jest wyłączony i nie będzie wywoływany.\nPrzeciągnij gniazda, aby utworzyć funkcjonalność.
)

(fn ConstructionScript
  (|CallParentFunction))