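; Melee enemy character that chases the player once a BP_BaseCharacter enters its proximity sense, and attacks in range.
; FollowPlayer loops AIMoveTo, a random attack montage and a cooldown, while the separate ZadajObrażenia event applies damage if the player is close, otherwise resumes the chase.
; Incoming damage updates and briefly reveals a health-bar widget.
; At zero health it calls BossPokonany once, plays death sound and montage, disables collision and destroys itself.
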(event OnComponentBeginOverlap(ZmyslBliskosci)
  (params (OverlappedComponent :type Primitive%20Component%20Object%20Reference) (OtherActor :type Actor%20Object%20Reference) (OtherComp :type Primitive%20Component%20Object%20Reference) (OtherBodyIndex :type Integer) (bFromSweep :type Boolean) (SweepResult :type Hit%20Result%20Structure%20%28by%20ref%29))
  (Utilities|Casting|CastToBP_BaseCharacter OtherActor)
  (Variables|Default|SetisSeeingPlayer? true)
  (CallFunction|FollowPlayer))

(event Custom|FollowPlayer
  (if (Variables|Default|GetcanAttack?)
    (AI|AIMoveTo self "0, 0, 0" (Game|GetPlayerCharacter 0) (Variables|Default|GetZasiegAtaku) false
      (:OnSuccess
        (if (Variables|Default|GetcanAttack?)
          (Variables|Default|SetcanAttack? false)
          (Components|Movement|StopMovementImmediately (Variables|Character|GetCharacterMovement))
          (Animation|PlayAnimMontage (Utilities|Select :Index (Math|Random|RandomIntegerinRange 0 1) :Option%200 (Variables|Default|GetAnimacjaAtaku) :Option%201 (Variables|Default|GetAnimacjaAtaku_2)) 1.0 "None")
          (Utilities|FlowControl|Delay 2.5)
          (Variables|Default|SetcanAttack? true)
          (CallFunction|FollowPlayer))))))

(event Custom|ZadajObrażenia
  (if (< (Transformation|GetDistanceTo (Game|GetPlayerCharacter 0)) (+ (Variables|Default|GetZasiegAtaku) (Variables|Default|GetSzerokosc%20Potwora)))
    (Game|Damage|ApplyDamage (Game|GetPlayerCharacter 0) (Variables|Default|GetObrazeniaPotwora) 0 0)
    (else
      (Variables|Default|SetcanAttack? true)
      (CallFunction|FollowPlayer))))

(event EventBeginPlay)

(event Collision|EventActorBeginOverlap
  (params (OtherActor :type Actor%20Object%20Reference)))

(event EventTick
  (params (DeltaSeconds :type Float%20%28single-precision%29)))

(event Game|Damage|EventAnyDamage
  (params (Damage :type Float%20%28single-precision%29) (DamageType :type Damage%20Type%20Object%20Reference) (InstigatedBy :type Controller%20Object%20Reference) (DamageCauser :type Actor%20Object%20Reference))
  (bind _pasekhp (Variables|Default|GetPasekHP))
  (Utilities|FlowControl|Sequence
    (:then_0
      (bind _output_get (Variables|Default|SetHealth (- (Variables|Default|GetHealth) Damage)))
      (bind _aswbp_health_bar (Utilities|Casting|CastToWBP_HealthBar (UserInterface|GetUserWidgetObject (Variables|Default|GetPasekHP))))
      (Progress|SetPercent (Variables|/Game/Enemies/WBP_HealthBar.WBP_HealthBar_C|GetProgressBar_0 _aswbp_health_bar) (/ (Variables|Default|GetHealth) (Variables|Default|GetMaxHealth)))
      (if (<= _output_get 0.0)
        (Utilities|FlowControl|DoOnce false
          (:Completed
            (Default|CallBossPokonany)
            (Variables|Default|SetcanAttack? false)
            (Components|Movement|StopMovementImmediately (Variables|Character|GetCharacterMovement))
            (Audio|PlaySoundatLocation (Variables|Default|GetDźwiękŚmierci) (Transformation|GetActorLocation) "0, 0, 0" 1.0 1.0 0.0 0 0 0 0)
            (Animation|PlayAnimMontage "/Game/Enemies/Animacje/DyingBackwardsEnemySmall_Montage.DyingBackwardsEnemySmall_Montage" 1.0 "None")
            (Collision|SetCollisionEnabled (Variables|Character|GetMesh) "NoCollision")
            (Utilities|FlowControl|Delay 4.2)
            (Components|SkeletalMesh|SetAnimInstanceClass (Variables|Character|GetMesh) 0)
            (Actor|DestroyActor)))))
    (:then_1
      (Development|SetHiddeninGame _pasekhp false false)
      (Utilities|FlowControl|RetriggerableDelay 2.0)
      (Development|SetHiddeninGame _pasekhp true false))))

(fn ConstructionScript)

(fn PrzelaczPasekBossa
  (params (Pokazac :type Boolean)))