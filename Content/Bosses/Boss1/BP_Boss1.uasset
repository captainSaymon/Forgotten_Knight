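; BP_Boss1 is a child boss Blueprint that manages the first boss's on-screen health bar.
; On BeginPlay it creates the health bar widget and stores it as a WBP_HealthBarBoss1.
; Its PrzelaczPasekBossa override calls the parent, then adds the bar to the viewport with a debug print.
; When hiding, it grants the player character extra MagicStones before removing the bar, so every hide call also gives that reward.
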(event EventBeginPlay
  (|CallParentFunction)
  (bind _returnvalue (UserInterface|CreateWidget (Variables|Default|GetKlasaPaskaBossa)))
  (bind _aswbp_health_bar_boss_1 (Utilities|Casting|CastToWBP_HealthBarBoss1 _returnvalue))
  (Variables|Default|SetPasekNaEkranieBossa _aswbp_health_bar_boss_1))

(event Collision|EventActorBeginOverlap
  (params (OtherActor :type Actor%20Object%20Reference))
  (|CallParentFunction OtherActor) ; Ten węzeł jest wyłączony i nie będzie wywoływany.\nPrzeciągnij gniazda, aby utworzyć funkcjonalność.
)

(event EventTick
  (params (DeltaSeconds :type Float%20%28single-precision%29))
  (|CallParentFunction DeltaSeconds) ; Ten węzeł jest wyłączony i nie będzie wywoływany.\nPrzeciągnij gniazda, aby utworzyć funkcjonalność.
)

(fn ConstructionScript
  (|CallParentFunction))

(fn PrzelaczPasekBossa
  (params (Pokazac :type Boolean))
  (bind _paseknaekraniebossa (Variables|Default|GetPasekNaEkranieBossa))
  (|CallParentFunction Pokazac)
  (if Pokazac
    (UserInterface|Viewport|AddtoViewport _paseknaekraniebossa 0)
    (Development|PrintString "FUNKCJA WYSWIETLA PASEK")
    (else
      (bind _asbp_base_character (Utilities|Casting|CastToBP_BaseCharacter (Game|GetPlayerCharacter 0)))
      (Variables|/Game/Blueprints/Player/BP_BaseCharacter.BP_BaseCharacter_C|SetMagicStones _asbp_base_character (+ (Variables|/Game/Blueprints/Player/BP_BaseCharacter.BP_BaseCharacter_C|GetMagicStones _asbp_base_character) 2))
      (Widget|RemovefromParent _paseknaekraniebossa))))