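; BP_Boss2 is the second boss enemy, a child Blueprint that relies on its parent for BeginPlay and boss bar toggling.
; On BeginPlay it creates a boss bar widget from KlasaPaskaBossa2, but sets PasekNaEkranieBossa2 to None instead of storing that widget.
; PrzelaczPasekBossa (toggle boss bar) only forwards Pokazac (show) to the parent.
; Its own nodes for adding and removing the widget are disconnected and never run.
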(event EventBeginPlay
  (|CallParentFunction)
  (bind _returnvalue (UserInterface|CreateWidget (Variables|Default|GetKlasaPaskaBossa2)))
  (Variables|Default|SetPasekNaEkranieBossa2 0))

(event Collision|EventActorBeginOverlap
  (params (OtherActor :type Actor%20Object%20Reference))
  (|CallParentFunction OtherActor) ; Ten węzeł jest wyłączony i nie będzie wywoływany.\nPrzeciągnij gniazda, aby utworzyć funkcjonalność.
)

(fn ConstructionScript
  (|CallParentFunction))

(fn PrzelaczPasekBossa
  (params (Pokazac :type Boolean))
  (|CallParentFunction Pokazac))