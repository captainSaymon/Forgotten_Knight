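; Small melee enemy character that chases and attacks the player once its pawn sensing spots them.
; FollowPlayer runs AI MoveTo, plays an attack montage, applies damage after it if the player is still close, then calls itself to repeat.
; Incoming damage lowers health, updates a health bar widget and, at zero, triggers a one-time death montage, disables collision and destroys the actor after a delay.
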(event OnSeePawn(PawnSensing)
  (params (Pawn :type Pawn%20Object%20Reference))
  (Variables|Default|SetisSeeingPlayer? true)
  (CallFunction|FollowPlayer))

(event Custom|FollowPlayer
  (if (Variables|Default|GetcanAttack?)
    (AI|AIMoveTo self "0, 0, 0" (Game|GetPlayerCharacter 0) 7e+01 false
      (:OnSuccess
        (if (Variables|Default|GetcanAttack?)
          (Variables|Default|SetcanAttack? false)
          (Components|Movement|StopMovementImmediately (Variables|Character|GetCharacterMovement))
          (bind _returnvalue (Animation|PlayAnimMontage (Variables|Default|GetAnimacjaAtaku) 1.0 "None"))
          (Utilities|FlowControl|Delay _returnvalue)
          (if (< (Transformation|GetDistanceTo (Game|GetPlayerCharacter 0)) 1.7e+02)
            (Game|Damage|ApplyDamage (Game|GetPlayerCharacter 0) (Variables|Default|GetObrazeniaPotwora) 0 0))
          (Variables|Default|SetcanAttack? true)
          (CallFunction|FollowPlayer))))))

(event EventBeginPlay)

(event Collision|EventActorBeginOverlap
  (params (OtherActor :type Actor%20Object%20Reference)))

(event EventTick
  (params (DeltaSeconds :type Float%20%28single-precision%29)))

(event Game|Damage|EventAnyDamage
  (params (Damage :type Float%20%28single-precision%29) (DamageType :type Damage%20Type%20Object%20Reference) (InstigatedBy :type Controller%20Object%20Reference) (DamageCauser :type Actor%20Object%20Reference))
  (bind _output_get (Variables|Default|SetHealth (- (Variables|Default|GetHealth) Damage)))
  (bind _aswbp_health_bar (Utilities|Casting|CastToWBP_HealthBar (UserInterface|GetUserWidgetObject (Variables|Default|GetPasekHP))))
  (Progress|SetPercent (Variables|/Game/Enemies/EnemiesSmall/WBP_HealthBar.WBP_HealthBar_C|GetProgressBar_0 _aswbp_health_bar) (/ (Variables|Default|GetHealth) (Variables|Default|GetMaxHealth)))
  (if (<= _output_get 0.0)
    (Utilities|FlowControl|DoOnce false
      (:Completed
        (Variables|Default|SetcanAttack? false)
        (Components|Movement|StopMovementImmediately (Variables|Character|GetCharacterMovement))
        (Animation|PlayAnimMontage "/Game/Enemies/EnemiesSmall/DyingBackwardsEnemySmall_Montage.DyingBackwardsEnemySmall_Montage" 1.0 "None")
        (Collision|SetCollisionEnabled (Variables|Character|GetMesh) "NoCollision")
        (Utilities|FlowControl|Delay 4.2)
        (Components|SkeletalMesh|SetAnimInstanceClass (Variables|Character|GetMesh) 0)
        (Actor|DestroyActor)))))

(fn ConstructionScript)